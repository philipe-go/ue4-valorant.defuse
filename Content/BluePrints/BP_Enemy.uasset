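; BP_Enemy is an enemy that idles, aims at nearby players and dies after taking enough projectile hits.
; While IsInCombat is set, Tick checks player distance and replays the looping aim animation within range.
; Two first-person projectile types deal different damage; surviving hits print HP, spawn Niagara blood and increase a "Hit" dynamic material parameter created in the Construction Script.
; At zero HP it clears IsInCombat and plays the death animation once.
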(event `self.ReceiveBeginPlay`
  ;[0.4138 1 0.1684] Begin Anim
  (`SkeletalMeshComponent.PlayAnimation` (`self.SK_Enemy`) "/Game/Animations/A_EnemyIdle.A_EnemyIdle" true)
  (set `self.Player` (`GameplayStatics.GetPlayerPawn` 0)))

(event `self.ReceiveTick`
  (params (DeltaSeconds :type "Float (single-precision)"))
  ;[0.9673 1 0.2732] Change Anim
  (if (and (`self.isInCombat`) (<= (`KismetMathLibrary.Vector_Distance` (`self.K2_GetActorLocation` (`self.Player`)) (`self.K2_GetActorLocation`)) 500.0))
    (`SkeletalMeshComponent.PlayAnimation` (`self.SK_Enemy`) "/Game/Animations/A_EnemyAim.A_EnemyAim" true)))

(event `self.ReceiveHit`
  (params (MyComp :type "PrimitiveComponent Object Reference") (Other :type "Actor Object Reference") (OtherComp :type "PrimitiveComponent Object Reference") (bSelfMoved :type Boolean) (HitLocation :type "Vector Structure") (HitNormal :type "Vector Structure") (NormalImpulse :type "Vector Structure") (Hit :type "HitResult Structure (by ref)"))
  (bind _hp (`self.HP`))
  (bind _dynmaterial (`self.DynMaterial`))
  ;[0.9688 0.2679 0.02018] Get Damage
  (cast `/Game/FirstPersonBP/Blueprints/FirstPersonProjectile` Other
    (:`then`
      (bind _output_get (set `self.HP` (- _hp 2))))
    (:`CastFailed`
      (cast `/Game/FirstPersonBP/Blueprints/FirstPersonProjectile2` Other)
      (set `self.HP` (- _hp 1))))
  (if (<= _output_get 0)
    (if (`self.isInCombat`)
      (set `self.isInCombat` false)
      (`SkeletalMeshComponent.PlayAnimation` (`self.SK_Enemy`) "/Game/Animations/A_EnemyDie.A_EnemyDie" false))
    (else
      (`KismetSystemLibrary.PrintString` (`KismetStringLibrary.Concat_StrStr` (`self.Name`) "HP = " (`KismetStringLibrary.Conv_IntToString` _output_get)))
      (`NiagaraFunctionLibrary.SpawnSystemAtLocation` "/Game/VFX/NS_EnemyBlood.NS_EnemyBlood" HitLocation (`KismetMathLibrary.Conv_VectorToRotator` (`SceneComponent.GetForwardVector` (`self.SK_Enemy`))))
      (bind _returnvalue (`MaterialInstanceDynamic.K2_GetScalarParameterValue` _dynmaterial "Hit"))
      (`MaterialInstanceDynamic.SetScalarParameterValue` _dynmaterial "Hit" (+ _returnvalue 0.25)))))

(fn `UserConstructionScript`
  (bind _returnvalue (`PrimitiveComponent.CreateDynamicMaterialInstance` (`self.SK_Enemy`) 1 null "None"))
  (set `self.DynMaterial` _returnvalue))