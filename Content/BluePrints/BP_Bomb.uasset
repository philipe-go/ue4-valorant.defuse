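; BP_Bomb is a countdown bomb that registers itself as BombTemp on an overlapping BP_Player.
; Until IsDefused is set externally, Tick prints the timer and lowers the dynamic material's "DEF" parameter by a fixed per-frame step.
; At zero it spawns explosion effects and sound, then destroys itself.
; When defused it sets DEF high and stops ticking; both outcomes print a restart hint.
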(event `self.ReceiveActorBeginOverlap`
  (params (OtherActor :type "Actor Object Reference"))
  ;[1 0.5765 0.1602] Player Overlap
  (bind _asbp_player (cast `/Game/BluePrints/BP_Player` OtherActor))
  (set `/Game/BluePrints/BP_Player.bombTemp` self _asbp_player))

(event `self.ReceiveTick`
  (params (DeltaSeconds :type "Float (single-precision)"))
  (bind _dynmaterial (`self.DynMaterial`))
  (bind _dynmaterial_2 (`self.DynMaterial`))
  ;[0.5016 0.1027 1] On Defuse
  (if (not (`self.isDefused`))
    (bind _output_get (set `self.Timer` (- (`self.Timer`) DeltaSeconds)))
    (`KismetSystemLibrary.PrintString` (`KismetStringLibrary.Concat_StrStr` "DEFUSE TIMER:" (`KismetStringLibrary.Conv_IntToString` (`KismetMathLibrary.FTrunc` _output_get))) true true (struct :`G` 0.66 :`B` 1.0 :`A` 1.0) 0.0)
    (bind _returnvalue (`MaterialInstanceDynamic.K2_GetScalarParameterValue` _dynmaterial "DEF"))
    (`MaterialInstanceDynamic.SetScalarParameterValue` _dynmaterial "DEF" (- _returnvalue 0.1))
    (if (<= _output_get 0.0)
      (`NiagaraFunctionLibrary.SpawnSystemAtLocation` "/Game/VFX/NS_BombExplode.NS_BombExplode" (`SceneComponent.K2_GetComponentLocation` (`self.SM_Bomb`)))
      (`KismetSystemLibrary.PrintString` "BOMB EXPLODED!")
      (`GameplayStatics.PlaySound2D` "/Game/StarterContent/Audio/Collapse01.Collapse01" 1.0 1.0 0.0 null null)
      (`self.K2_DestroyActor`)
      (`KismetSystemLibrary.PrintString` "RESTART THE GAME BY SHOOTING THE \"X\"" true true (struct :`R` 1.0 :`G` 0.036923 :`B` 0.857892 :`A` 1.0) 5.0 :!label _label))
    (else
      (`KismetSystemLibrary.PrintString` "BOMB DEFUSED!" true true (struct :`R` 0.371468 :`G` 1.0 :`A` 1.0))
      (`MaterialInstanceDynamic.K2_GetScalarParameterValue` _dynmaterial_2 "DEF")
      (`MaterialInstanceDynamic.SetScalarParameterValue` _dynmaterial_2 "DEF" 4.0)
      (`self.SetActorTickEnabled` false)
      (goto _label))))

(fn `UserConstructionScript`
  (bind _returnvalue (`PrimitiveComponent.CreateDynamicMaterialInstance` (`self.SM_Bomb`) 1 null "None"))
  (set `self.DynMaterial` _returnvalue))